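; Blueprint function library for Secpho Companion that formats timestamps and shortens strings for display.
; TimeStampToText shows hour:minute when the date's day number matches today's, ignoring month and year, and otherwise prefixes day/month with no separator.
; It zero-pads minutes and months, and returns empty text if the result equals "0/00".
; CutoutString truncates strings longer than a given length and appends an ellipsis.
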(fn TimeStamptoText
  (params (date :type Date%20Time%20Compressed%20Structure))
  (bind (_day _month _hour _min) (Utilities|Struct|BreakDateTimeCompressed date))
  (bind _returnvalue (Math|DateTime|Now))
  (bind _returnvalue_2 (>= _month 10))
  (bind _day_2 (Math|DateTime|BreakDateTime _returnvalue))
  (bind _returnvalue_3 (>= _min 10))
  (bind _result (Utilities|Text|FormatText "{0}/{1}" _day _month))
  (bind _result_2 (Utilities|Text|FormatText "{0}:{1}" _hour _min))
  (bind _result_3 (Utilities|Text|FormatText "{0}:0{1}" _hour _min))
  (bind _result_4 (Utilities|Text|FormatText "{0}/0{1}" _day _month))
  (bind _returnvalue_4 (Math|Conversions|ToByte(Integer) _day_2))
  (bind _returnvalue_5 (select _returnvalue_2 _result _result_4))
  (bind _returnvalue_6 (select _returnvalue_3 _result_2 _result_3))
  (bind _returnvalue_7 (== _day _returnvalue_4))
  (bind _returnvalue_8 (Utilities|String|ToString(Text) _returnvalue_5))
  (bind _returnvalue_9 (Utilities|String|ToString(Text) _returnvalue_6))
  (bind _returnvalue_10 (Utilities|String|Append _returnvalue_8 "    " _returnvalue_9))
  (bind _returnvalue_11 (Utilities|Text|ToText(String) _returnvalue_10))
  (bind _returnvalue_12 (select _returnvalue_7 _returnvalue_6 _returnvalue_11))
  (return (select (Utilities|Enum|Equal(Enum) (Utilities|Text|MakeLiteralText "0/00") _returnvalue_12) "" _returnvalue_12)))

(fn CutoutString
  (params (string :type String) (len :type Integer))
  (return (select (> (Utilities|String|Len string) len) (Utilities|String|Append (Utilities|String|Left string len) "...") string)))