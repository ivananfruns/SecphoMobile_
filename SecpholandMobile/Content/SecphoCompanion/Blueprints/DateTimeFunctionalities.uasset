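; Date and time helper functions for SecphoCompanion, working on a compact DateTimeCompressed struct that stores byte fields with the year offset from 2000.
; Two formatters build hour:minute text with zero-padded minutes and day/month text with a zero-padded month.
; The other helpers expand the struct to DateTime to convert it, add minutes and repack, or compare two values.
; The comparison labelled ">" returns true when Val1 is earlier than Val2.
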(fn TimetoHourText
  (params (compressedTime :type Date%20Time%20Compressed%20Structure))
  (bind (_day _month _hour _min) (Utilities|Struct|BreakDateTimeCompressed compressedTime))
  (return (select (>= _min 10) (Utilities|Text|FormatText "{0}:{1}" _hour _min) (Utilities|Text|FormatText "{0}:0{1}" _hour _min))))

(fn TimetoDayText
  (params (DateTimeCompressed :type Date%20Time%20Compressed%20Structure%20%28by%20ref%29))
  (bind (_day _month) (Utilities|Struct|BreakDateTimeCompressed DateTimeCompressed))
  (return (select (>= _month 10) (Utilities|Text|FormatText "{0}/{1}" _day _month) (Utilities|Text|FormatText "{0}/0{1}" _day _month))))

(fn TimeAddMinutestoTime
  (params (date :type Date%20Time%20Compressed%20Structure) (Min :type Integer))
  (bind (_day _month _hour _min _año20000) (Utilities|Struct|BreakDateTimeCompressed date))
  (bind _returnvalue (Math|Timespan|MakeTimespan 0 0 Min))
  (bind _returnvalue_2 (Math|Conversions|ToInteger(Byte) _año20000))
  (bind _returnvalue_3 (Math|Conversions|ToInteger(Byte) _min))
  (bind _returnvalue_4 (Math|Conversions|ToInteger(Byte) _hour))
  (bind _returnvalue_5 (Math|Conversions|ToInteger(Byte) _day))
  (bind _returnvalue_6 (Math|Conversions|ToInteger(Byte) _month))
  (bind _returnvalue_7 (+ _returnvalue_2 2000))
  (bind _returnvalue_8 (Math|DateTime|MakeDateTime _returnvalue_7 _returnvalue_6 _returnvalue_5 _returnvalue_4 _returnvalue_3))
  (bind _returnvalue_9 (+ _returnvalue_8 _returnvalue))
  (bind (_year _month_2 _day_2 _hour_2 _minute) (Math|DateTime|BreakDateTime _returnvalue_9))
  (return (Utilities|Struct|MakeDateTimeCompressed (Math|Conversions|ToByte(Integer) _day_2) (Math|Conversions|ToByte(Integer) _month_2) (Math|Conversions|ToByte(Integer) _hour_2) (Math|Conversions|ToByte(Integer) _minute) (Math|Conversions|ToByte(Integer) (- _year 2000)))))

(fn TimeOperator>
  (params (val1_ :type Date%20Time%20Compressed%20Structure) (val2_ :type Date%20Time%20Compressed%20Structure))
  (bind (_day _month _hour _min _año20000) (Utilities|Struct|BreakDateTimeCompressed val2_))
  (bind (_day_2 _month_2 _hour_2 _min_2 _año20000_2) (Utilities|Struct|BreakDateTimeCompressed val1_))
  (return (< (Math|DateTime|MakeDateTime (+ (Math|Conversions|ToInteger(Byte) _año20000_2) 2000) (Math|Conversions|ToInteger(Byte) _month_2) (Math|Conversions|ToInteger(Byte) _day_2) (Math|Conversions|ToInteger(Byte) _hour_2) (Math|Conversions|ToInteger(Byte) _min_2)) (Math|DateTime|MakeDateTime (+ (Math|Conversions|ToInteger(Byte) _año20000) 2000) (Math|Conversions|ToInteger(Byte) _month) (Math|Conversions|ToInteger(Byte) _day) (Math|Conversions|ToInteger(Byte) _hour) (Math|Conversions|ToInteger(Byte) _min)))))

(fn UncompressDateTime
  (params (DateTimeCompressed :type Date%20Time%20Compressed%20Structure%20%28by%20ref%29))
  (bind (_day _month _hour _min _año20000) (Utilities|Struct|BreakDateTimeCompressed DateTimeCompressed))
  (return (Math|DateTime|MakeDateTime (+ (Math|Conversions|ToInteger(Byte) _año20000) 2000) (Math|Conversions|ToInteger(Byte) _month) (Math|Conversions|ToInteger(Byte) _day) (Math|Conversions|ToInteger(Byte) _hour) (Math|Conversions|ToInteger(Byte) _min))))