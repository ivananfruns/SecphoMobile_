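; Player controller for the Secpho companion app, handling login and requests for events, companies, friends, user profiles and chat.
; Requests go to PuzzleGameMode, most carrying the username and GameInstance security token, while the UssingBypass flag skips login and substitutes hard-coded test data.
; Successful login creates the MenuBar and fetches events and friends to fill it.
; Company, profile, chat history and message receive events are empty here.
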(event Custom|RetrieveEvents
  ;[1 1 1] Eventos
  (if (Variables|Default|GetussingBypass)
    (|ByPassEvents)
    (else
      (Default|RetreiveEventList (.AsPuzzle%20Game%20Mode (Utilities|Casting|CastToPuzzleGameMode (Game|GetGameMode))) (Utilities|Struct|BreakUserInfo_Public (Variables|Default|Getuserinfo_Public)) (Variables|/Game/SecphoCompanion/Blueprints/PuzzleGameInstace.PuzzleGameInstace_C|GetsecurityToken (.AsPuzzle%20Game%20Instace (Utilities|Casting|CastToPuzzleGameInstace (Game|GetGameInstance))))))))

(event Custom|SendMessageChat
  (params (Friend%20Name :type String) (message :type String))
  ;[1 1 1] Chat
  (if (Variables|Default|GetussingBypass)
    (|ByPassChat)
    (else
      (Default|SendMessageChat (.AsPuzzle%20Game%20Mode (Utilities|Casting|CastToPuzzleGameMode (Game|GetGameMode))) (Utilities|Struct|BreakUserInfo_Public (Variables|Default|Getuserinfo_Public)) (Variables|/Game/SecphoCompanion/Blueprints/PuzzleGameInstace.PuzzleGameInstace_C|GetsecurityToken (.AsPuzzle%20Game%20Instace (Utilities|Casting|CastToPuzzleGameInstace (Game|GetGameInstance)))) Friend%20Name message))))

(event Custom|ReceiveEmpresa
  (params (EmpresaInfo :type Empresa%20Structure))
  ;[1 1 1] UserEmpresa / Empresa
)

(event Custom|Receive%20User%20info
  (params (UserInfo :type User%20Info%20Public%20Structure))
  ;[1 1 1] User Infor Public
)

(event Custom|Retrieve%20User%20info
  (params (UserNameToFind :type String))
  ;[1 1 1] User Infor Public
  (if (Variables|Default|GetussingBypass)
    (|ByPassUserPublic)
    (else
      (Default|RetrieveUserInfo (.AsPuzzle%20Game%20Mode (Utilities|Casting|CastToPuzzleGameMode (Game|GetGameMode))) (Utilities|Struct|BreakUserInfo_Public (Variables|Default|Getuserinfo_Public)) (Variables|/Game/SecphoCompanion/Blueprints/PuzzleGameInstace.PuzzleGameInstace_C|GetsecurityToken (.AsPuzzle%20Game%20Instace (Utilities|Casting|CastToPuzzleGameInstace (Game|GetGameInstance)))) UserNameToFind))))

(event Custom|ReceiveMessageChat
  (params (SenderName :type Name) (Text :type String) (timeStamp :type Date%20Time%20Compressed%20Structure))
  ;[1 1 1] Chat
)

(event Custom|ConnectedToSocket
  ;[1 1 1] SocketConnection
  (Utilities|IsValid (Game|Player|GetPlayerPawn 0)
    (:Is%20Valid
      (bind _returnvalue (UserInterface|CreateWidget "/Game/SecphoCompanion/Widgets/loggin.loggin_C"))
      (UserInterface|Viewport|AddtoViewport _returnvalue 0))))

(event Custom|ReceiveEvents
  (params (EventosSecpholand :type Array%20of%20Evento%20En%20Secpholand%20Structures))
  ;[1 1 1] Eventos
  (Variables|/Game/SecphoCompanion/Widgets/MenuBar.MenuBar_C|Seteventos (Variables|Default|GetMenuBar) EventosSecpholand))

(event Custom|Retrieve%20Friends
  ;[1 1 1] FriendList
  (if (Variables|Default|GetussingBypass)
    (|BypassFriends)
    (else
      (Default|RetrieveFriends (.AsPuzzle%20Game%20Mode (Utilities|Casting|CastToPuzzleGameMode (Game|GetGameMode))) (Utilities|Struct|BreakUserInfo_Public (Variables|Default|Getuserinfo_Public)) (Variables|/Game/SecphoCompanion/Blueprints/PuzzleGameInstace.PuzzleGameInstace_C|GetsecurityToken (.AsPuzzle%20Game%20Instace (Utilities|Casting|CastToPuzzleGameInstace (Game|GetGameInstance))))))))

(event Custom|ReturnLoggin
  (params (Succesfull :type Boolean) (userinfo_Private :type User%20Info%20Private%20Structure) (userinfo_Public :type User%20Info%20Public%20Structure))
  ;[1 1 1] Loggin
  (bind _foundwidgets (Widget|GetAllWidgetsOfClass "/Game/SecphoCompanion/Widgets/loggin.loggin_C" true))
  (Default|ReturnLoggin (Utilities|Array|Get(acopy) _foundwidgets) Succesfull)
  (if Succesfull
    (Variables|Default|Setuserinfo_Private userinfo_Private)
    (Variables|Default|Setuserinfo_Public userinfo_Public)
    (bind _returnvalue (UserInterface|CreateWidget "/Game/SecphoCompanion/Widgets/MenuBar.MenuBar_C"))
    (bind _output_get (Variables|Default|SetMenuBar _returnvalue))
    (UserInterface|Viewport|AddtoViewport _output_get 0)
    (CallFunction|RetrieveEvents)
    (CallFunction|RetrieveFriends)))

(event Custom|Receive%20Friends
  (params (FriendUsernames :type Array%20of%20Names) (FriendConnectionStates :type Array%20of%20playerConnectionState%20Enums :default "NewEnumerator0") (lastMessage :type Array%20of%20Strings) (lastMessageTimestamp :type Array%20of%20Date%20Time%20Compressed%20Structures) (Mensajes%20por%20leer :type Array%20of%20Integers) (Names :type Array%20of%20Names) (URLPerfiles :type Array%20of%20Strings) (pendingInvitations :type Array%20of%20Booleans) (YouAreSender :type Array%20of%20Booleans))
  ;[1 1 1] FriendList
  (bind _output_get (Variables|/Game/SecphoCompanion/Widgets/MenuBar.MenuBar_C|SetChatHot (Variables|Default|GetMenuBar) FriendUsernames))
  (for (_ _array_index) _output_get
    (Utilities|Array|Add (Variables|/Game/SecphoCompanion/Widgets/MenuBar.MenuBar_C|GetChatCold (Variables|Default|GetMenuBar)) (Utilities|Struct|MakeChat (Utilities|Array|Get(acopy) Names _array_index) (Utilities|Array|MakeArray (Utilities|Array|Get(acopy) lastMessage _array_index)) (Utilities|Array|MakeArray false) (Utilities|Array|MakeArray (Utilities|Array|Get(acopy) lastMessageTimestamp _array_index)) (Utilities|Array|Get(acopy) Mensajes%20por%20leer _array_index) false (Utilities|Array|Get(acopy) FriendConnectionStates _array_index) (Utilities|Array|Get(acopy) URLPerfiles _array_index) (Utilities|Array|Get(acopy) pendingInvitations _array_index) (Utilities|Array|Get(acopy) YouAreSender _array_index)))))

(event Custom|LogginAtempt
  (params (username :type String) (Pw :type String))
  ;[1 1 1] Loggin
  (if (Variables|Default|GetussingBypass)
    (CallFunction|ReturnLoggin true)
    (else
      (Default|RetreiveLoggin (.AsPuzzle%20Game%20Mode (Utilities|Casting|CastToPuzzleGameMode (Game|GetGameMode))) username Pw))))

(event Custom|RetrieveEmpresa
  (params (EmpresaName :type String))
  ;[1 1 1] UserEmpresa / Empresa
  (if (Variables|Default|GetussingBypass)
    (|bypassempresa)
    (else
      (Default|RetrieveEmpresa (.AsPuzzle%20Game%20Mode (Utilities|Casting|CastToPuzzleGameMode (Game|GetGameMode))) (Utilities|Struct|BreakUserInfo_Public (Variables|Default|Getuserinfo_Public)) (Variables|/Game/SecphoCompanion/Blueprints/PuzzleGameInstace.PuzzleGameInstace_C|GetsecurityToken (.AsPuzzle%20Game%20Instace (Utilities|Casting|CastToPuzzleGameInstace (Game|GetGameInstance)))) EmpresaName))))

(event Custom|ReceiveChatHistory
  (params (Chat :type Chat%20Structure%20%28by%20ref%29))
  ;[1 1 1] Chat History
)

(event Custom|DisconecteddFromSocket
  ;[1 1 1] SocketConnection
)

(event Custom|RetrieveChatHistory
  (params (Friend%20Name :type String))
  ;[1 1 1] Chat History
  (if (Variables|Default|GetussingBypass)
    (|ByPassChathistory)
    (else
      (Default|RetrieveChatHistory (.AsPuzzle%20Game%20Mode (Utilities|Casting|CastToPuzzleGameMode (Game|GetGameMode))) (Utilities|Struct|BreakUserInfo_Public (Variables|Default|Getuserinfo_Public)) (Variables|/Game/SecphoCompanion/Blueprints/PuzzleGameInstace.PuzzleGameInstace_C|GetsecurityToken (.AsPuzzle%20Game%20Instace (Utilities|Casting|CastToPuzzleGameInstace (Game|GetGameInstance)))) Friend%20Name))))

(event EventBeginPlay
  (Networking|SwitchHasAuthority
    (:Authority
      (if (Variables|Default|GetussingBypass)
        (CallFunction|ConnectedtoSocket)))))

(fn ConstructionScript
  (if (Variables|Default|GetussingBypass)
    (CallFunction|ConnectedtoSocket)))